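; BP_Cube is a cube actor meant to spawn beneath the player character as they move, though its BeginPlay and Tick events are empty.
; Disconnected logic would snap the cube below the player and store that location.
; A second disconnected chain would spawn another BP_Cube below the player once movement passes a distance threshold, using DoOnce, then destroy itself after a short delay.
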(event `self.ReceiveBeginPlay`
  ;[1 1 1] 正方体在人物正下方生成
)

(event `self.ReceiveTick`
  (params (DeltaSeconds :type "Float (single-precision)"))
  ;[1 1 1] 判断位移量是否大于100，大于则生成物体
)

(fn `UserConstructionScript`)