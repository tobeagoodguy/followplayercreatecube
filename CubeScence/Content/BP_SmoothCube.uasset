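; BP_SmoothCube is an actor with a cube that appears and changes position when a player-tagged actor enters its trigger box.
; On begin overlap the cube becomes visible and jumps to the EndLocation component's world position.
; On end overlap it hides and returns to StartLocation.
; Both moves are instant SetWorldLocation calls without sweep or interpolation, despite the "Smooth" in the name.
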(event `self.Box.OnComponentBeginOverlap`
  (params (OverlappedComponent :type "PrimitiveComponent Object Reference") (OtherActor :type "Actor Object Reference") (OtherComp :type "PrimitiveComponent Object Reference") (OtherBodyIndex :type Integer) (bFromSweep :type Boolean) (SweepResult :type "HitResult Structure (by ref)"))
  (bind _cube (`self.Cube`))
  ;[1 1 1] 重叠时显示方块，移动到End位置
  (if (`self.ActorHasTag` OtherActor "player")
    (`SceneComponent.SetVisibility` _cube true false)
    (`SceneComponent.K2_SetWorldLocation` _cube (`SceneComponent.K2_GetComponentLocation` (`self.EndLocation`)) false false)))

(event `self.Box.OnComponentEndOverlap`
  (params (OverlappedComponent :type "PrimitiveComponent Object Reference") (OtherActor :type "Actor Object Reference") (OtherComp :type "PrimitiveComponent Object Reference") (OtherBodyIndex :type Integer))
  (bind _cube (`self.Cube`))
  ;[1 1 1] 无重叠时隐藏方块，方块移动到初始位置
  (if (`self.ActorHasTag` OtherActor "player")
    (`SceneComponent.SetVisibility` _cube false false)
    (`SceneComponent.K2_SetWorldLocation` _cube (`SceneComponent.K2_GetComponentLocation` (`self.StartLocation`)) false false)))

(fn `UserConstructionScript`)